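; BP_Dynamic is a dynamic physics object that registers itself as a rigid body in the BP_BulletWorld simulation.
; On BeginPlay, after a zero-length delay, it finds the first BulletWorld actor and passes itself with friction, restitution and mass.
; It stores and prints the returned body ID.
; Pressing Space uses that ID to apply an upward force through BulletWorld.
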(event `self.ReceiveBeginPlay`
  (`KismetSystemLibrary.Delay` 0.0)
  (bind _outactors (`GameplayStatics.GetAllActorsOfClass` "/Game/BP_BulletWorld.BP_BulletWorld_C"))
  (bind _output_get (set `self.BulletWorld` (`|GetArrayItem` _outactors)))
  (bind _id (`TestActor.AddRigidBody` _output_get self (`self.Friction`) (`self.Restitution`) (`self.Mass`)))
  (bind _output_get_2 (set `self.ID` _id))
  (`KismetSystemLibrary.PrintString` (`KismetStringLibrary.Conv_IntToString` _output_get_2)))

(event `Key|SpaceBar`
  (params (Key :type "Key Structure"))
  (:`Pressed`
    (`TestActor.AddForce` (`self.BulletWorld`) (`self.ID`) (0.0 0.0 1000.0) (0.0 0.0 0.0))))

(event `self.ReceiveTick`
  (params (DeltaSeconds :type "Float (single-precision)")))

(fn `UserConstructionScript`)