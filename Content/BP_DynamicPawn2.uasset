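; BP_DynamicPawn2 is a debug pawn for testing networked rigid-body physics through BP_BulletWorld.
; Shortly after BeginPlay the server registers the pawn as a body and multicasts its ID, which clients map to their own local body ID.
; Space applies an upward force to the local body and sends the server ID to Jump for the server's body.
; Debug keys trigger server spawning, manual physics stepping and test jumps.
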(event Custom|jump
  (params (ServerID :type Integer))
  ;[0.15 0.15 0.15 0.5] VERY SIMPLE INPUT scheme for debugging, implement input queue later
  (Class|TestActor|AddForce (Variables|Default|GetBulletWorld) ServerID "0.000000,0.000000,1000.000000" "0, 0, 0"))

(event Custom|MC_jump
  ;[0.15 0.15 0.15 0.5] VERY SIMPLE INPUT scheme for debugging, implement input queue later
  (if (not (Ability|HasAuthority))
    (Class|TestActor|AddForce (Variables|Default|GetBulletWorld) (Variables|Default|GetID) "0.000000,0.000000,100000.000000" "0, 0, 0")))

(event Custom|MC_TellClients
  (params (ServerID :type Integer))
  (bind _id (Variables|Default|GetID))
  (if (not (Networking|IsServer))
    ;[0.15 0.15 0.15 0.5] On clients, spawn and add association between server ID and local ID
    (bind _output_get (CallFunction|GetBulletWorld))
    (bind _id_2 (Class|TestActor|AddRigidBody _output_get self (Variables|Default|GetFriction) (Variables|Default|GetRestitution) (Variables|Default|GetMass)))
    (CallFunction|SetID _id_2)
    (Utilities|Map|Add (Variables|/Script/BulletPhysicsEngine.TestActor|GetServerIdToClientId (Variables|Default|GetBulletWorld)) ServerID _id)
    (Variables|Default|SetServerID ServerID)
    (if (not (Ability|HasAuthority))
      (Development|PrintString (Utilities|String|Append "Spawned something! Server ID: " (Utilities|String|ToString(Integer) ServerID) " and Local ID: " (Utilities|String|ToString(Integer) _id))))))

(event Custom|SR_SpawnThingOnServer
  ;[0.15 0.15 0.15 0.5] Spawn something on the server
  (Game|SpawnActorfromClass "BP_DynamicPawn2_C" (Math|Transform|MakeTransform "0, 0, 0") "Undefined" "MultiplyWithRoot" 0 0))

(event EventBeginPlay
  (Utilities|FlowControl|Delay 0.5)
  (if (Networking|IsServer)
    ;[0.15 0.15 0.15 0.5] If server, spawn and tell others to spawn with server id
    (bind _output_get (CallFunction|GetBulletWorld))
    (bind _id (Class|TestActor|AddRigidBody _output_get self (Variables|Default|GetFriction) (Variables|Default|GetRestitution) (Variables|Default|GetMass)))
    (bind _output_get_2 (Variables|Default|SetServerID _id))
    (CallFunction|MCTellClients _output_get_2)))

(event Input|KeyboardEvents|DebugKeyC
  (params (Key :type Key%20Structure :default "None") (ActionValue :type Input%20Action%20Value%20Structure))
  ;[0.15 0.15 0.15 0.5] executes on server
  (:Pressed
    (CallFunction|Jump)))

(event Input|KeyboardEvents|DebugKeyS
  (params (Key :type Key%20Structure :default "None") (ActionValue :type Input%20Action%20Value%20Structure))
  ;[0.15 0.15 0.15 0.5] Spawn something on the server
  (:Pressed
    (CallFunction|SRSpawnThingonServer)))

(event Input|KeyboardEvents|DebugKeyD
  (params (Key :type Key%20Structure :default "None") (ActionValue :type Input%20Action%20Value%20Structure))
  (:Pressed
    (Class|TestActor|StepPhysics (Variables|Default|GetBulletWorld) 0.01666)))

(event Input|KeyboardEvents|SpaceBar
  (params (Key :type Key%20Structure :default "None"))
  ;[0.15 0.15 0.15 0.5] VERY SIMPLE INPUT scheme for debugging, implement input queue later
  (:Pressed
    (Class|TestActor|AddForce (Variables|Default|GetBulletWorld) (Variables|Default|GetID) "0.000000,0.000000,1000.000000" "0, 0, 0")
    (CallFunction|Jump (Variables|Default|GetServerID))))

(fn ConstructionScript)

(fn SetID
  (params (Int :type Integer))
  (bind _output_get (Variables|Default|SetID Int))
  (Development|PrintString (Utilities|String|Append "Local ID has been set to " (Utilities|String|ToString(Integer) _output_get))))

(fn GetBulletWorld
  (bind _outactors (Actor|GetAllActorsOfClass "/Game/BP_BulletWorld.BP_BulletWorld_C"))
  (bind _output_get (Variables|Default|SetBulletWorld (Utilities|Array|Get(acopy) _outactors)))
  (return _output_get))